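; BowlingPin_BP is a bowling pin that detects when it gets knocked by a ball or another pin.
; On a mesh hit from a BowlingBall_BP or BowlingPin_BP, it compares the normal impulse's magnitude against MinForceOfImpact.
; The first sufficient impact sets WasHit and calls the PinWasHit event dispatcher, so the pin reports only once while that flag stays set.
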(event `self.StaticMeshComponent.OnComponentHit`
  (params (HitComponent :type "PrimitiveComponent Object Reference") (OtherActor :type "Actor Object Reference") (OtherComp :type "PrimitiveComponent Object Reference") (NormalImpulse :type "Vector Structure") (Hit :type "HitResult Structure (by ref)"))
  (bind _returnvalue (`GameplayStatics.GetObjectClass` OtherActor))
  (castclass `/Game/Blueprints/BowlingBall_BP` _returnvalue
    (:`then`
      _)
    (:`CastFailed`
      (castclass `/Game/Blueprints/BowlingPin_BP` _returnvalue)))
  (if (`self.bWasHit`)
    _
    (elif (>= (`KismetMathLibrary.VSize` NormalImpulse) (`self.MinForceOfImpact`))
      (set `self.bWasHit` true)
      (`self.PinWasHit`))))

(event `self.ReceiveBeginPlay`
  (`parent.ReceiveBeginPlay`))

(fn `UserConstructionScript`)